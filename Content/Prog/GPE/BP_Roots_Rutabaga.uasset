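; Root vegetable physics prop whose sphere gets a random impulse whenever it hits something, making it bounce erratically.
; On BeginPlay, it silences its sounds and sets the Root mesh from the vegetable enum, with a dynamic material instance.
; Three vibe sounds play after random delays, each calling Vibe to restart the cycle, which also adds another sound manager each time.
; Unconnected material-swap and splash-effect nodes never run.
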(event `self.Sphere.OnComponentHit`
  (params (HitComponent :type "PrimitiveComponent Object Reference") (OtherActor :type "Actor Object Reference") (OtherComp :type "PrimitiveComponent Object Reference") (NormalImpulse :type "Vector Structure") (Hit :type "HitResult Structure (by ref)"))
  ;[0 0.7408 1] Random bounces on hit
  (`PrimitiveComponent.AddImpulseAtLocation` (`self.Sphere`) (`KismetMathLibrary.MakeVector` (`KismetMathLibrary.RandomFloatInRange` (`self.Min Force On X`) (`self.Max Force On X`)) (`KismetMathLibrary.RandomFloatInRange` (`self.Min Force On Y`) (`self.Max Force On Y`)) (`KismetMathLibrary.RandomFloatInRange` (`self.Min force On Z`) (`self.Max force On Z`))) (`self.K2_GetActorLocation`) "None"))

(event `self.ReceiveBeginPlay`
  (bind _returnvalue (`KismetMathLibrary.RandomFloatInRange` 5.0 60.0))
  (bind _root (`self.Root`))
  (`AudioComponent.Stop` (`self.Throw`))
  (`AudioComponent.Stop` (`self.VibeSound`))
  (`AudioComponent.Stop` (`self.VibeSound_2`))
  (`AudioComponent.Stop` (`self.VibeSound_3`))
  ;[0 0.7408 1] Get mesh from roots
  (`|ExecutionSequence`
    (:`then_0`
      (`AddComponent|NODE_AddBP_SoundManager-2` :!label _label)
      (`|ExecutionSequence`
        (:`then_0`
          (`KismetSystemLibrary.Delay` _returnvalue)
          (`AudioComponent.Play` (`self.VibeSound`) 0.0))
        (:`then_1`
          (`KismetSystemLibrary.Delay` _returnvalue)
          (`AudioComponent.Play` (`self.VibeSound_2`) 0.0))
        (:`then_2`
          (`KismetSystemLibrary.Delay` _returnvalue)
          (`AudioComponent.Play` (`self.VibeSound_3`) 0.0)))
      (`self.Vibe`))
    (:`then_1`
      (switch `/Game/Prog/Enum_Root` (`self.Enum Roots`)
        (:`NewEnumerator0`
          (set `self.Index` 0))
        (:`NewEnumerator1`
          (set `self.Index` 1))
        (:`NewEnumerator5`
          (set `self.Index` 2))
        (:`NewEnumerator2`
          (set `self.Index` 3))
        (:`NewEnumerator3`
          (set `self.Index` 4))
        (:`NewEnumerator4`
          (set `self.Index` 5)))
      (`StaticMeshComponent.SetStaticMesh` _root (`|GetArrayItem` (`self.Mesh Contenu`) (`self.Index`)))
      (`PrimitiveComponent.CreateDynamicMaterialInstance` _root 0 null "None"))))

(event `Vibe`
  (goto _label))

(fn `UserConstructionScript`)