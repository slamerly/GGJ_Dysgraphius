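; BP_Potion is a potion actor whose appearance follows a Potion enum of six color and shape variants.
; On BeginPlay it converts the enum to an index, picks the matching static mesh from the MeshsPotion array, then assigns a stopper (BOUCHON) material by slot name.
; The Rose torus variant reuses the Rouge triangle's stopper slot and material.
; The construction script is empty, so this setup runs only at BeginPlay.
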(event `self.ReceiveBeginPlay`
  (bind _meshpotion (`self.MeshPotion`))
  (bind _index (`self.index`))
  (switch `/Game/Prog/Enum_Potion` (`self.Potion`)
    (:`NewEnumerator0`
      (set `self.index` 0))
    (:`NewEnumerator1`
      (set `self.index` 1))
    (:`NewEnumerator2`
      (set `self.index` 2))
    (:`NewEnumerator3`
      (set `self.index` 3))
    (:`NewEnumerator4`
      (set `self.index` 4))
    (:`NewEnumerator5`
      (set `self.index` 5)))
  (`StaticMeshComponent.SetStaticMesh` _meshpotion (`|GetArrayItem` (`self.MeshsPotion`) _index))
  (switch `int` _index
    (:`0`
      (`PrimitiveComponent.SetMaterialByName` _meshpotion "BOUCHON" "/Game/Art/Materials/Bouchon.Bouchon" :!label _label))
    (:`1`
      (`PrimitiveComponent.SetMaterialByName` _meshpotion "BOUCHON_002" "/Game/Art/Materials/BOUCHON_002.BOUCHON_002"))
    (:`2`
      (`PrimitiveComponent.SetMaterialByName` _meshpotion "BOUCHON_004" "/Game/Art/Materials/BOUCHON_004.BOUCHON_004"))
    (:`3`
      (`PrimitiveComponent.SetMaterialByName` _meshpotion "BOUCHON_003" "/Game/Art/Materials/BOUCHON_003.BOUCHON_003"))
    (:`4`
      (goto _label))
    (:`5`
      (`PrimitiveComponent.SetMaterialByName` _meshpotion "BOUCHON_001" "/Game/Art/Materials/BOUCHON_001.BOUCHON_001"))))

(fn `UserConstructionScript`)