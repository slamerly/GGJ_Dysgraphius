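; BP_SpawnCustomer is a spawner actor that sends a wave of twenty AI customers toward a shop.
; On BeginPlay, a delayed loop spawns each BP_AI_Customer at the spawner's transform, using a random delay between configurable minimum and maximum values.
; Each customer is added to TriggerRef's ClientArray, given the shop location and told to move there.
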(event `self.ReceiveBeginPlay`
  (`/Game/Prog/Macros/M_ForEachLoopWithDelay.For Loop With Delay` 0 19 (`KismetMathLibrary.RandomFloatInRange` (`self.Min Delay Between Customer`) (`self.Max Delay Between Customer`))
    (:`Loop Body`
      (bind _returnvalue (`|SpawnActorFromClass` "/Game/Prog/GPE/BP_AI_Customer.BP_AI_Customer_C" (`self.GetTransform`) "Undefined" "OverrideRootScale" null null))
      (`KismetArrayLibrary.Array_Add` (`/Game/Prog/GPE/BP_Trigger_Client.Client Array` (`self.Trigger ref`)) _returnvalue)
      (set `/Game/Prog/GPE/BP_AI_Customer.Shop Location` (`self.Shop Location`) _returnvalue)
      (`/Game/Prog/GPE/BP_AI_Customer.Move To Shop` _returnvalue))))

(fn `UserConstructionScript`)