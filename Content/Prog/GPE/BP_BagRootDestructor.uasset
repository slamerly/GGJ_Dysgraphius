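; BP_BagRootDestructor is a trigger box that destroys BP_Roots_Impulse actors of one enum type, commented as the "bad guy", when they overlap it.
; On overlap it makes player 0 drop their held object, then stops the root sphere's physics and snaps it to the box's location.
; It plays a sound through BPSoundManager and destroys the root after a short delay.
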(event `self.Box.OnComponentBeginOverlap`
  (params (OverlappedComponent :type "PrimitiveComponent Object Reference") (OtherActor :type "Actor Object Reference") (OtherComp :type "PrimitiveComponent Object Reference") (OtherBodyIndex :type Integer) (bFromSweep :type Boolean) (SweepResult :type "HitResult Structure (by ref)"))
  (bind _asbp_roots_impulse (cast `/Game/Prog/GPE/BP_Roots_Impulse` OtherActor))
  ;[1 1 1] Si bad guy
  (if (`|EnumEquality` (`/Game/Prog/GPE/BP_Roots_Impulse.Enum Roots` _asbp_roots_impulse) "NewEnumerator4")
    (bind _asbp_player (cast `/Game/Prog/Core/BP_Player` (`GameplayStatics.GetPlayerPawn` 0)))
    (`/Game/Prog/Core/BP_Player.Drop Object` _asbp_player)
    (bind _sphere (`/Game/Prog/GPE/BP_Roots_Impulse.Sphere` _asbp_roots_impulse))
    ;[1 1 1] interdire de bouger
    (`PrimitiveComponent.SetSimulatePhysics` _sphere false)
    (`SceneComponent.K2_SetWorldLocation` _sphere (`SceneComponent.K2_GetComponentLocation` (`self.Box`)) false false)
    (`/Game/Prog/Core/BP_SoundManager.PlaySFX` (`self.BP_SoundManager`) "NewEnumerator2" self)
    (`KismetSystemLibrary.Delay` 0.2)
    (`self.K2_DestroyActor` OtherActor)))

(fn `UserConstructionScript`)