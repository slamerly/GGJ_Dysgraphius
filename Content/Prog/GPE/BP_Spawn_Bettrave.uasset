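; BP_Spawn_Bettrave is a spawner that keeps creating BP_Roots_Betrave actors during play.
; From BeginPlay, SpawnRoots waits a random delay between the min and max spawn times, spawns one actor, then calls itself to repeat indefinitely.
; Each spawn takes the world transform of one of five scene components, picked at random.
; Some leftover root-enum logic is disconnected and never runs.
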(event `self.ReceiveBeginPlay`
  (`self.Spawn Roots`))

(event `Spawn Roots`
  (`KismetSystemLibrary.Delay` (`KismetMathLibrary.RandomFloatInRange` (`self.Min Time Before Spawn`) (`self.Max Time Before Spawn`)))
  (`|SpawnActorFromClass` "/Game/Prog/GPE/BP_Roots_Betrave.BP_Roots_Betrave_C" (`SceneComponent.K2_GetComponentToWorld` (select `int` (`KismetMathLibrary.RandomIntegerInRange` 0 4) :`0` (`self.Scene`) :`1` (`self.Scene1`) :`2` (`self.Scene2`) :`3` (`self.Scene3`) :`4` (`self.Scene4`))) "Undefined" "OverrideRootScale" null null)
  (`self.Spawn Roots`))

(fn `UserConstructionScript`)