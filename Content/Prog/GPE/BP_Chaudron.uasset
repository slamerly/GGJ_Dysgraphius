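; Cauldron actor that collects actors entering its box trigger as ingredients on a spinning water component.
; On BeginPlay it caches the water's child components as ingredient slots; Tick advances the water's yaw.
; For each true availability entry, overlap records the actor, rescales it and snaps it to the slot at its new index.
; An optional reset button's activation only clears the slot component list and prints a message.
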(event `self.ReceiveBeginPlay`
  (bind _resetbutton (`self.ResetButton`))
  (`self.Init`)
  (`/Engine/EditorBlueprintResources/StandardMacros.IsValid` _resetbutton
    (:`Is Valid`
      (add `/Game/Prog/GPE/BP_ResetChaudron.On Activation` _resetbutton (delegate `ResetIngredient`)))))

(event `ResetIngredient`
  ;[1 1 1] Reset
  (`KismetArrayLibrary.Array_Clear` (`self.PositionIngredients`))
  (`KismetSystemLibrary.PrintString` "Reset"))

(event `self.ReceiveTick`
  (params (DeltaSeconds :type "Float (single-precision)"))
  (bind _eau (`self.Eau`))
  (bind (_returnvalue_roll _returnvalue_pitch _returnvalue_yaw) (`KismetMathLibrary.BreakRotator` (`SceneComponent.K2_GetComponentRotation` _eau)))
  (`SceneComponent.K2_SetWorldRotation` _eau (`KismetMathLibrary.MakeRotator` 0.0 0.0 (+ _returnvalue_yaw (`self.SpeedRotation`))) false false))

(event `self.Box.OnComponentBeginOverlap`
  (params (OverlappedComponent :type "PrimitiveComponent Object Reference") (OtherActor :type "Actor Object Reference") (OtherComp :type "PrimitiveComponent Object Reference") (OtherBodyIndex :type Integer) (bFromSweep :type Boolean) (SweepResult :type "HitResult Structure (by ref)"))
  (for _array_element (`self.PositionDispo`)
    (if _array_element
      (bind _returnvalue (`KismetArrayLibrary.Array_Add` (`self.IngredientsIn`) OtherActor))
      (`self.SetActorScale3D` OtherActor (`SceneComponent.K2_GetComponentScale` (`self.Position`)))
      (`self.K2_AttachToComponent` OtherActor (`|GetArrayItem` (`self.PositionIngredients`) _returnvalue) "None" "SnapToTarget" "SnapToTarget" "SnapToTarget" true)
      (`KismetArrayLibrary.Array_Set` (`self.PositionDispo`) _returnvalue true))))

(fn `Init`
  (for _array_element (`SceneComponent.GetChildrenComponents` (`self.Eau`) false)
    (`KismetArrayLibrary.Array_Add` (`self.PositionIngredients`) _array_element)))

(fn `UserConstructionScript`)