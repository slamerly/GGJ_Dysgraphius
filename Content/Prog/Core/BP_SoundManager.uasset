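; Sound manager that plays the game's one-shot effects for vegetables, customers, the cauldron and other gameplay events.
; PlaySFX switches on a sound-type value and plays the matching SFX asset at the location of the passed Actor.
; PlayMusic plays at the first player controller's location, but has no sound asset assigned.
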(fn `PlayMusic`
  (`GameplayStatics.PlaySoundAtLocation` null (`Actor.K2_GetActorLocation` (`GameplayStatics.GetPlayerController` 0)) (struct) 1.0 1.0 0.0 null null null null))

(fn `PlaySFX`
  (params (SoundFonction :type "/Game/Prog/Enum_SoundFonction Enum" :default "NewEnumerator0") (Actor :type "Actor Object Reference"))
  (bind _returnvalue (`Actor.K2_GetActorLocation` Actor))
  (switch `/Game/Prog/Enum_SoundFonction` SoundFonction
    (:`NewEnumerator0`
      (`GameplayStatics.PlaySoundAtLocation` "/Game/Sound/SFX/SFX_Legume_mechant_spawn.SFX_Legume_mechant_spawn" _returnvalue (struct) 1.0 1.0 0.0 null null null null))
    (:`NewEnumerator1`
      (`GameplayStatics.PlaySoundAtLocation` "/Game/Sound/SFX/SFX_Legume_mechant_Vibe.SFX_Legume_mechant_Vibe" _returnvalue (struct) 1.0 1.0 0.0 null null null null))
    (:`NewEnumerator2`
      (`GameplayStatics.PlaySoundAtLocation` "/Game/Sound/SFX/SFX_Legume_mechant_die.SFX_Legume_mechant_die" _returnvalue (struct) 1.0 1.0 0.0 null null null null))
    (:`NewEnumerator7`
      (`GameplayStatics.PlaySoundAtLocation` "/Game/Sound/SFX/SFX_Legume_sortie_terre.SFX_Legume_sortie_terre" _returnvalue (struct) 1.0 1.0 0.0 null null null null))
    (:`NewEnumerator8`
      (`GameplayStatics.PlaySoundAtLocation` "/Game/Sound/SFX/SFX_Attraper.SFX_Attraper" _returnvalue (struct) 1.0 1.0 0.0 null null null null))
    (:`NewEnumerator9`
      (`GameplayStatics.PlaySoundAtLocation` "/Game/Sound/SFX/SFX_Client_blablabla.SFX_Client_blablabla" _returnvalue (struct) 1.0 1.0 0.0 null null null null))
    (:`NewEnumerator10`
      (`GameplayStatics.PlaySoundAtLocation` "/Game/Sound/SFX/SFX_Client_heureux.SFX_Client_heureux" _returnvalue (struct) 1.0 1.0 0.0 null null null null))
    (:`NewEnumerator11`
      (`GameplayStatics.PlaySoundAtLocation` "/Game/Sound/SFX/SFX_Client_colere.SFX_Client_colere" _returnvalue (struct) 1.0 1.0 0.0 null null null null))
    (:`NewEnumerator12`
      (`GameplayStatics.PlaySoundAtLocation` "/Game/Sound/SFX/SFX_Client_bonne_commande.SFX_Client_bonne_commande" _returnvalue (struct) 1.0 1.0 0.0 null null null null))
    (:`NewEnumerator13`
      (`GameplayStatics.PlaySoundAtLocation` "/Game/Sound/SFX/SFX_GameOverLost.SFX_GameOverLost" _returnvalue (struct) 1.0 1.0 0.0 null null null null))
    (:`NewEnumerator14`
      (`GameplayStatics.PlaySoundAtLocation` "/Game/Sound/SFX/SFX_Lancer_3.SFX_Lancer_3" _returnvalue (struct) 1.0 1.0 0.0 null null null null))
    (:`NewEnumerator15`
      (`GameplayStatics.PlaySoundAtLocation` "/Game/Sound/SFX/SFX_Legume_dans_marmite.SFX_Legume_dans_marmite" _returnvalue (struct) 1.0 1.0 0.0 null null null null))
    (:`NewEnumerator16`
      (`GameplayStatics.PlaySoundAtLocation` "/Game/Sound/SFX/SFX_Legume_drop.SFX_Legume_drop" _returnvalue (struct) 1.0 1.0 0.0 null null null null))
    (:`NewEnumerator17`
      (`GameplayStatics.PlaySoundAtLocation` "/Game/Sound/SFX/SFX_LEgume_lancer.SFX_LEgume_lancer" _returnvalue (struct) 1.0 1.0 0.0 null null null null))
    (:`NewEnumerator18`
      (`GameplayStatics.PlaySoundAtLocation` "/Game/Sound/SFX/SFX_Legume_vibe.SFX_Legume_vibe" _returnvalue (struct) 1.0 1.0 0.0 null null null null))
    (:`NewEnumerator19`
      (`GameplayStatics.PlaySoundAtLocation` "/Game/Sound/SFX/SFX_Legume_Vibe_2.SFX_Legume_Vibe_2" _returnvalue (struct) 1.0 1.0 0.0 null null null null))
    (:`NewEnumerator20`
      (`GameplayStatics.PlaySoundAtLocation` "/Game/Sound/SFX/SFX_Legume_vibe_3.SFX_Legume_vibe_3" _returnvalue (struct) 1.0 1.0 0.0 null null null null))
    (:`NewEnumerator21`
      (`GameplayStatics.PlaySoundAtLocation` "/Game/Sound/SFX/SFX_Levier.SFX_Levier" _returnvalue (struct) 1.0 1.0 0.0 null null null null))
    (:`NewEnumerator22`
      (`GameplayStatics.PlaySoundAtLocation` "/Game/Sound/SFX/SFX_Marmite_bonne_recette.SFX_Marmite_bonne_recette" _returnvalue (struct) 1.0 1.0 0.0 null null null null))
    (:`NewEnumerator23`
      (`GameplayStatics.PlaySoundAtLocation` "/Game/Sound/SFX/SFX_Marmite_explosion.SFX_Marmite_explosion" _returnvalue (struct) 1.0 1.0 0.0 null null null null))
    (:`NewEnumerator24`
      (`GameplayStatics.PlaySoundAtLocation` "/Game/Sound/SFX/SFX_slpash.SFX_slpash" _returnvalue (struct) 1.0 1.0 0.0 null null null null))
    (:`NewEnumerator25`
      (`GameplayStatics.PlaySoundAtLocation` "/Game/Sound/SFX/SFX_Sonette.SFX_Sonette" _returnvalue (struct) 1.0 1.0 0.0 null null null null))))